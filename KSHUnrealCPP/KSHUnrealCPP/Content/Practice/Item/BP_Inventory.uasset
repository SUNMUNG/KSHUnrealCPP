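; BP_Inventory is a practice inventory Blueprint that holds item data and gives the player a toggleable inventory screen.
; On BeginPlay it creates a WBP_Inventory widget for player 0, sizes its ItemStruct array to ten slots, and passes itself to the widget's LoadInventory.
; The I key adds the widget to the viewport, or removes it if it is already visible.
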(event `self.ReceiveBeginPlay`
  (bind _returnvalue (`|CreateWidget` "/Game/UI/WBP_Inventory.WBP_Inventory_C" (`GameplayStatics.GetPlayerController` 0)))
  (set `self.Inventory` _returnvalue)
  (`KismetArrayLibrary.Array_Resize` (`self.ItemStruct`) 10)
  (`/Game/UI/WBP_Inventory.LoadInventory` (`self.Inventory`) self))

(event `Key|I`
  (params (Key :type "Key Structure"))
  (bind _inventory (`self.Inventory`))
  (:`Pressed`
    (if (`Widget.IsVisible` _inventory)
      (`Widget.RemoveFromParent` _inventory)
      (else
        (`UserWidget.AddToViewport` _inventory 0)))))