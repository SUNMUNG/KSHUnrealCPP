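; BP_DummyEnemy is a dummy enemy that reports the damage it receives, with no health or reaction logic in its graphs.
; Its AnyDamage event prints the damage amount, then the display names of the damage type, instigator and damage causer.
; The name lines are assembled with BuildStringInteger, passing each name as the suffix and leaving the integer input unset.
; The construction script is empty.
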(event `self.ReceiveAnyDamage`
  (params (Damage :type "Float (single-precision)") (DamageType :type "DamageType Object Reference") (InstigatedBy :type "Controller Object Reference") (DamageCauser :type "Actor Object Reference"))
  (`KismetSystemLibrary.PrintString` (`KismetStringLibrary.BuildString_Double` "" "Damage :" Damage))
  (`KismetSystemLibrary.PrintString` (`KismetStringLibrary.BuildString_Int` "Damage Type: " "" 0 (`KismetSystemLibrary.GetDisplayName` DamageType)))
  (`KismetSystemLibrary.PrintString` (`KismetStringLibrary.BuildString_Int` "Damage Instigator: " "" 0 (`KismetSystemLibrary.GetDisplayName` InstigatedBy)))
  (`KismetSystemLibrary.PrintString` (`KismetStringLibrary.BuildString_Int` "Damage Causer: " "" 0 (`KismetSystemLibrary.GetDisplayName` DamageCauser))))

(fn `UserConstructionScript`)